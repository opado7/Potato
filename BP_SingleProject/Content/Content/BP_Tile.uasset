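; BP_Tile is a clickable grid tile actor that highlights under the cursor and reacts to bombs.
; Hover swaps the Plane material unless it shows TileHighlight or gold, and clicking sends the tile's location to the player controller's MoveTileHighlightMessage.
; When a BP_Bomb overlaps its collision, it waits briefly, spawns an explosion, destroys the bomb and passes its first tag as an integer to the player character's CallExplosive.
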(event OnBeginCursorOver(Cube)
  (params (TouchedComponent :type Primitive%20Component%20Object%20Reference))
  (bind _plane (Variables|Default|GetPlane))
  (bind _returnvalue (Rendering|Material|GetMaterial _plane 0))
  (if (not (or (== _returnvalue "/Game/Materials/Interface/TileHighlight.TileHighlight") (== _returnvalue "/Game/StarterContent/Materials/M_Metal_Gold.M_Metal_Gold")))
    (Rendering|Material|SetMaterial _plane 0 "/Game/Materials/Interface/TileHighlight_Inst_gridHighlight.TileHighlight_Inst_gridHighlight")))

(event OnEndCursorOver(Cube)
  (params (TouchedComponent :type Primitive%20Component%20Object%20Reference))
  (bind _plane (Variables|Default|GetPlane))
  (bind _returnvalue (Rendering|Material|GetMaterial _plane 0))
  (if (not (or (== _returnvalue "/Game/Materials/Interface/TileHighlight.TileHighlight") (== _returnvalue "/Game/StarterContent/Materials/M_Metal_Gold.M_Metal_Gold")))
    (Rendering|Material|SetMaterial _plane 0 "/Engine/BufferVisualization/AmbientOcclusion.AmbientOcclusion")))

(event OnClicked(Cube)
  (params (TouchedComponent :type Primitive%20Component%20Object%20Reference) (ButtonPressed :type Key%20Structure :default "None"))
  (bind _cube (Variables|Default|GetCube))
  (bind _returnvalue (Transformation|GetWorldLocation _cube))
  (Development|PrintString (Utilities|String|ToString(Vector) _returnvalue))
  (Class|BPIFHighlight|MoveTileHighlight(Message) (Game|GetPlayerController 0) _returnvalue))

(event OnComponentBeginOverlap(tilecollision)
  (params (OverlappedComponent :type Primitive%20Component%20Object%20Reference) (OtherActor :type Actor%20Object%20Reference) (OtherComp :type Primitive%20Component%20Object%20Reference) (OtherBodyIndex :type Integer) (bFromSweep :type Boolean) (SweepResult :type Hit%20Result%20Structure%20%28by%20ref%29))
  (bind _asbp_bomb (Utilities|Casting|CastToBP_Bomb OtherActor))
  (Utilities|FlowControl|Delay 1.0)
  (bind _returnvalue (Effects|SpawnEmitteratLocation "/Game/StarterContent/Particles/P_Explosion.P_Explosion" (Transformation|GetWorldLocation (Variables|/Game/Content/BP_Bomb.BP_Bomb_C|GetCube _asbp_bomb)) "0, 0, 0" "2.500000,2.500000,2.500000" false))
  (Actor|DestroyActor _asbp_bomb)
  (if (Utilities|IsValid _returnvalue)
    (bind _asbp_top_down_character (Utilities|Casting|CastToBP_TopDownCharacter (Game|Player|GetPlayerPawn 0)))
    (Default|CallExplosive _asbp_top_down_character (Math|Conversions|ToInteger(Byte) (Utilities|String|ToString(Name) (Utilities|Array|Get(acopy) (Variables|Actor|GetTags)))))))

(event EventBeginPlay)

(event Collision|EventActorBeginOverlap
  (params (OtherActor :type Actor%20Object%20Reference)))

(event EventTick
  (params (DeltaSeconds :type Float%20%28single-precision%29)))

(fn ConstructionScript)

(fn Iszero
  (params (NewParam :type Vector))
  (bind _returnvalue (== (.y NewParam) 0.0))
  (if (== (.x NewParam) 0.0)
    (if _returnvalue
      (return "0, 0, 0"))
    (elif _returnvalue
      (return (Math|Vector|MakeVector (.x NewParam) 0.0 0.0))
      (else
        (return (Math|Vector|MakeVector (.x NewParam) (.y NewParam) 0.0))))))