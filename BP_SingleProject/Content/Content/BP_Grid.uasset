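; BP_Grid is an actor that spawns a Row by Column grid of BP_Tile actors when play begins.
; MakeGrid uses nested loops to place tiles at Cellsize intervals, composed with the actor's transform so the grid follows its placement.
; Click converts a given position to cell indices using a hardcoded 200-unit size, ignoring the actor's transform, and only prints them.
; The construction-script build and static-mesh component variants are disconnected.
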(event EventBeginPlay
  (CallFunction|MakeGrid))

(event Collision|EventActorBeginOverlap
  (params (OtherActor :type Actor%20Object%20Reference)))

(event EventTick
  (params (DeltaSeconds :type Float%20%28single-precision%29)))

(fn ConstructionScript)

(fn MakeGrid
  (for _index (range 0 (- (Variables|Default|GetRow) 1))
    (for _index_2 (range 0 (- (Variables|Default|GetColumn) 1))
      (Utilities|FlowControl|FlipFlop
        (:A
          _)
        (:B
          _))
      (Game|SpawnActorfromClass "/Game/BP_Tile.BP_Tile_C" (Math|Transform|MakeTransform (.location (Math|Transform|ComposeTransforms (Math|Transform|MakeTransform (Math|Vector|MakeVector (* _index_2 (Variables|Default|GetCellsize)) (* _index (Variables|Default|GetCellsize)) 0.0)) (Transformation|GetActorTransform))) "0, 0, 0" "1.000000,1.000000,1.000000") "Undefined" 0 0))))

(fn Click
  (params (Position :type Vector))
  (bind _returnvalue (/ Position "200.000000,200.000000,1.000000"))
  (bind (_x _y) (Math|Vector|BreakVector _returnvalue))
  (Development|PrintString (Utilities|String|Append (Utilities|String|ToString(Integer) (Math|Float|Floor _x)) ", " (Utilities|String|ToString(Integer) (Math|Float|Floor _y)))))