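; BP_Bomb is a bomb actor that explodes one second after its Spawn event fires.
; On BeginPlay it binds Spawn_Event to Spawn, and that event stores the received CubeNum before the delay.
; It then plays a scaled-up explosion emitter at the Cube component, destroys itself and passes CubeNum to the player's BP_TopDownCharacter through CallExplosive.
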(event Custom|Spawn_Event
  (params (Cube_Num :type Integer))
  (Variables|Default|SetCube_Num Cube_Num)
  (Utilities|FlowControl|Delay 1.0)
  (Effects|SpawnEmitteratLocation "/Game/StarterContent/Particles/P_Explosion.P_Explosion" (Transformation|GetWorldLocation (Variables|Default|GetCube)) "0, 0, 0" "2.500000,2.500000,2.500000" false)
  (Actor|DestroyActor)
  (bind _asbp_top_down_character (Utilities|Casting|CastToBP_TopDownCharacter (Game|GetPlayerCharacter 0)))
  (Default|CallExplosive _asbp_top_down_character (Variables|Default|GetCube_Num)))

(event Collision|EventActorBeginOverlap
  (params (OtherActor :type Actor%20Object%20Reference)))

(event EventTick
  (params (DeltaSeconds :type Float%20%28single-precision%29)))

(event EventBeginPlay
  (EventDispatchers|BindEventtoSpawn (delegate Custom|Spawn_Event)))

(fn ConstructionScript)