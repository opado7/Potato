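; BP_Hammer is a moving mallet hazard that deals damage, intended as lethal, to the player pawn on overlap.
; Its SpawnHam event sets a short lifespan, then uses the passed Go position to choose an X or Y travel direction, rolling the mesh a quarter turn for X.
; A Gate opened by that event lets Tick sweep the mesh along at constant, frame-rate-independent speed.
; Older movement and timeline nodes are left disconnected.
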(event OnComponentBeginOverlap(S_Mallet_tlvmeddjw_lod0)
  (params (OverlappedComponent :type Primitive%20Component%20Object%20Reference) (OtherActor :type Actor%20Object%20Reference) (OtherComp :type Primitive%20Component%20Object%20Reference) (OtherBodyIndex :type Integer) (bFromSweep :type Boolean) (SweepResult :type Hit%20Result%20Structure%20%28by%20ref%29))
  (bind _returnvalue (Game|Player|GetPlayerPawn 0))
  ;[1 1 1] 망치랑 충돌 시 사망
  (if (== OtherActor _returnvalue)
    (Game|Damage|ApplyDamage _returnvalue 1e+02 0 0)))

(event Custom|Spawn_Hammer
  (params (go :type Vector))
  (bind _s_mallet_tlvmeddjw_lod0 (Variables|Default|GetS_Mallet_tlvmeddjw_lod0))
  (bind _returnvalue (Transformation|GetWorldRotation _s_mallet_tlvmeddjw_lod0))
  (Actor|SetLifeSpan 3.0)
  (if (or (< (.x go) -5e+02) (> (.x go) 4e+02))
    (Transformation|SetWorldRotation _s_mallet_tlvmeddjw_lod0 (Math|Rotator|MakeRotator (+ (.roll _returnvalue) 9e+01) (.pitch _returnvalue) (.yaw _returnvalue)) false false)
    (if (< (.x go) -5e+02)
      (Variables|Default|SetX 1.0)
      (Utilities|FlowControl|Gate true) ; enters at Open
      (else
        (Variables|Default|SetX -1.0)
        (Utilities|FlowControl|Gate true) ; enters at Open
      ))
    (elif (< (.y go) 1e+03)
      (Variables|Default|SetY 1.0)
      (Utilities|FlowControl|Gate true) ; enters at Open
      (else
        (Variables|Default|SetY -1.0)
        (Utilities|FlowControl|Gate true) ; enters at Open
      ))))

(event EventBeginPlay
  (EventDispatchers|BindEventtoSpawnHam (delegate Custom|Spawn_Hammer)))

(event EventTick
  (params (DeltaSeconds :type Float%20%28single-precision%29))
  (Utilities|FlowControl|Gate true
    (:Exit
      (Transformation|SetWorldLocation (Variables|Default|GetS_Mallet_tlvmeddjw_lod0) (+ (* (* 1.2e+03 DeltaSeconds) (Math|Vector|MakeVector (Variables|Default|GetX) (Variables|Default|GetY) 0.0)) (Transformation|GetWorldLocation (Variables|Default|GetS_Mallet_tlvmeddjw_lod0))) true false))))

(fn ConstructionScript)