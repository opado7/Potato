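; Grid tile actor that reacts to cursor hover, bombs and the player.
; Hovering swaps the plane's material unless it is highlighted or gold, so the current material acts as tile state.
; An overlapping bomb explodes after a delay, is destroyed, and passes the tile's numeric tag to the player's CallExplosive.
; While the player overlaps a gold tile, a Tick-driven gate steadily raises the game instance's MadnessBar.
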(event OnComponentEndOverlap(tilecollision)
  (params (OverlappedComponent :type Primitive%20Component%20Object%20Reference) (OtherActor :type Actor%20Object%20Reference) (OtherComp :type Primitive%20Component%20Object%20Reference) (OtherBodyIndex :type Integer))
  (Utilities|Casting|CastToBP_TopDownCharacter OtherActor)
  (if (== (Rendering|Material|GetMaterial (Variables|Default|GetPlane) 0) "/Game/StarterContent/Materials/M_Metal_Gold.M_Metal_Gold")
    (Utilities|FlowControl|Gate true) ; enters at Close
  ))

(event OnBeginCursorOver(Cube)
  (params (TouchedComponent :type Primitive%20Component%20Object%20Reference))
  (bind _plane (Variables|Default|GetPlane))
  (bind _returnvalue (Rendering|Material|GetMaterial _plane 0))
  (if (not (or (== _returnvalue "/Game/Materials/Interface/TileHighlight.TileHighlight") (== _returnvalue "/Game/StarterContent/Materials/M_Metal_Gold.M_Metal_Gold")))
    (Rendering|Material|SetMaterial (Variables|Default|GetPlane) 0 "/Game/Materials/Interface/TileHighlight_Inst_gridHighlight.TileHighlight_Inst_gridHighlight")))

(event OnEndCursorOver(Cube)
  (params (TouchedComponent :type Primitive%20Component%20Object%20Reference))
  (bind _plane (Variables|Default|GetPlane))
  (bind _returnvalue (Rendering|Material|GetMaterial _plane 0))
  (if (not (or (== _returnvalue "/Game/Materials/Interface/TileHighlight.TileHighlight") (== _returnvalue "/Game/StarterContent/Materials/M_Metal_Gold.M_Metal_Gold")))
    (Rendering|Material|SetMaterial (Variables|Default|GetPlane) 0 "/Engine/BufferVisualization/AmbientOcclusion.AmbientOcclusion")))

(event OnComponentBeginOverlap(tilecollision)
  (params (OverlappedComponent :type Primitive%20Component%20Object%20Reference) (OtherActor :type Actor%20Object%20Reference) (OtherComp :type Primitive%20Component%20Object%20Reference) (OtherBodyIndex :type Integer) (bFromSweep :type Boolean) (SweepResult :type Hit%20Result%20Structure%20%28by%20ref%29))
  (bind _asbp_bomb (Utilities|Casting|CastToBP_Bomb OtherActor)
    (:then
      (Utilities|FlowControl|Delay 1.0)
      (bind _returnvalue (Effects|SpawnEmitteratLocation "/Game/StarterContent/Particles/P_Explosion.P_Explosion" (Transformation|GetWorldLocation (Variables|/Game/Content/Actor/BP_Bomb.BP_Bomb_C|GetCube _asbp_bomb)) "0, 0, 0" "2.500000,2.500000,2.500000"))
      (Actor|DestroyActor _asbp_bomb)
      (if (Utilities|IsValid _returnvalue)
        (bind _asbp_top_down_character (Utilities|Casting|CastToBP_TopDownCharacter (Game|Player|GetPlayerPawn 0)))
        (Default|CallExplosive _asbp_top_down_character (Math|Conversions|ToInteger(Byte) (Utilities|String|ToString(Name) (Utilities|Array|Get(acopy) (Variables|Actor|GetTags)))))))
    (:CastFailed
      (Utilities|Casting|CastToBP_TopDownCharacter OtherActor)
      (if (== (Rendering|Material|GetMaterial (Variables|Default|GetPlane) 0) "/Game/StarterContent/Materials/M_Metal_Gold.M_Metal_Gold")
        (Utilities|FlowControl|Gate true) ; enters at Open
      ))))

(event EventBeginPlay
  (for _index (range 0 0)
    _))

(event EventTick
  (params (DeltaSeconds :type Float%20%28single-precision%29))
  (Utilities|FlowControl|Gate true
    (:Exit
      (bind _asbp_instance (Utilities|Casting|CastToBP_Instance (Game|GetGameInstance)))
      (Variables|/Game/TopDown/Blueprints/BP_Instance.BP_Instance_C|SetMadness_Bar _asbp_instance (+ (Variables|/Game/TopDown/Blueprints/BP_Instance.BP_Instance_C|GetMadness_Bar _asbp_instance) (/ DeltaSeconds 5e+01))))))

(event Collision|EventActorBeginOverlap
  (params (OtherActor :type Actor%20Object%20Reference)))

(fn ConstructionScript)