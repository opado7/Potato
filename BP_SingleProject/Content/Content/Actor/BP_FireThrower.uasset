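; BP_FireThrower is a hazard actor that raises the player's madness while the player pawn stands inside its Capsule.
; Capsule begin and end overlaps with the player pawn open and close a Gate on Tick.
; While the gate is open, each tick adds a scaled DeltaSeconds to MadnessBar on BP_Instance, the game instance, so the gain is frame-rate independent.
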(event OnComponentBeginOverlap(Capsule)
  (params (OverlappedComponent :type Primitive%20Component%20Object%20Reference) (OtherActor :type Actor%20Object%20Reference) (OtherComp :type Primitive%20Component%20Object%20Reference) (OtherBodyIndex :type Integer) (bFromSweep :type Boolean) (SweepResult :type Hit%20Result%20Structure%20%28by%20ref%29))
  (if (== OtherActor (Game|Player|GetPlayerPawn 0))
    (Utilities|FlowControl|Gate true) ; enters at Open
  ))

(event OnComponentEndOverlap(Capsule)
  (params (OverlappedComponent :type Primitive%20Component%20Object%20Reference) (OtherActor :type Actor%20Object%20Reference) (OtherComp :type Primitive%20Component%20Object%20Reference) (OtherBodyIndex :type Integer))
  (if (== (Game|Player|GetPlayerPawn 0) OtherActor)
    (Utilities|FlowControl|Gate true) ; enters at Close
  ))

(event EventBeginPlay)

(event EventTick
  (params (DeltaSeconds :type Float%20%28single-precision%29))
  (Utilities|FlowControl|Gate true
    (:Exit
      (bind _asbp_instance (Utilities|Casting|CastToBP_Instance (Game|GetGameInstance)))
      (Variables|/Game/TopDown/Blueprints/BP_Instance.BP_Instance_C|SetMadness_Bar _asbp_instance (+ (Variables|/Game/TopDown/Blueprints/BP_Instance.BP_Instance_C|GetMadness_Bar _asbp_instance) (/ DeltaSeconds 5e+01))))))

(fn ConstructionScript)