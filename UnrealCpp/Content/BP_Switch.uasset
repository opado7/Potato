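; BP_Switch is an overlap-triggered switch that turns a list of other actors on and off.
; When its Cube begins or ends overlap, it loops through the Actors array and sends DoPlayMessage true or false to each actor implementing BPI_PlayObj.
; The interface decouples it from target classes; unreachable older loops that set play flags directly on LeftRight and NewVar remain in the graph.
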(event OnComponentBeginOverlap(Cube)
  (params (OverlappedComponent :type Primitive%20Component%20Object%20Reference) (OtherActor :type Actor%20Object%20Reference) (OtherComp :type Primitive%20Component%20Object%20Reference) (OtherBodyIndex :type Integer) (bFromSweep :type Boolean) (SweepResult :type Hit%20Result%20Structure%20%28by%20ref%29))
  (for _array_element (Variables|Default|GetActors)
    (if (Utilities|DoesObjectImplementInterface _array_element "/Game/Tools/BPI_PlayObj.BPI_PlayObj_C")
      (Class|BPIPlayObj|DoPlay(Message) _array_element true))))

(event OnComponentEndOverlap(Cube)
  (params (OverlappedComponent :type Primitive%20Component%20Object%20Reference) (OtherActor :type Actor%20Object%20Reference) (OtherComp :type Primitive%20Component%20Object%20Reference) (OtherBodyIndex :type Integer))
  (bind _array_element (Utilities|Array|ForEachLoopwithBreak (Variables|Default|GetActors))
    (:LoopBody
      (if (Utilities|DoesObjectImplementInterface _array_element "/Game/Tools/BPI_PlayObj.BPI_PlayObj_C")
        (Class|BPIPlayObj|DoPlay(Message) _array_element false)))))

(event EventBeginPlay)

(event Collision|EventActorBeginOverlap
  (params (OtherActor :type Actor%20Object%20Reference)))

(event EventTick
  (params (DeltaSeconds :type Float%20%28single-precision%29)))

(fn ConstructionScript)