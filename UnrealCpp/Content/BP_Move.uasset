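; BP_Move is a Blueprint that slides its static mesh back and forth along its relative X axis while play is enabled.
; Each Tick raises or lowers XPos by delta time, flipping the Right flag when it reaches the positive or negative limit.
; XPos is applied as a per-frame offset, so it acts as a ramping, frame-rate-dependent velocity.
; DoPlay sets the Isplay flag that gates the motion and always returns false.
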(event EventTick
  (params (DeltaSeconds :type Float%20%28single-precision%29))
  (if (Variables|Default|Getisplay)
    (if (Variables|Default|GetRight)
      (bind _output_get (Variables|Default|SetX_pos (+ (Variables|Default|GetX_pos) DeltaSeconds)))
      (Transformation|AddRelativeLocation (Variables|Default|GetStaticMesh) (Math|Vector|MakeVector _output_get 0.0 0.0) false false)
      (if (>= (Variables|Default|GetX_pos) 2.0)
        (Variables|Default|SetRight false))
      (else
        (bind _output_get_2 (Variables|Default|SetX_pos (- (Variables|Default|GetX_pos) DeltaSeconds)))
        (Transformation|AddRelativeLocation (Variables|Default|GetStaticMesh) (Math|Vector|MakeVector _output_get_2 0.0 0.0) false false)
        (if (<= (Variables|Default|GetX_pos) -2.0)
          (Variables|Default|SetRight true))))))

(fn ConstructionScript)

(fn DoPlay
  (params (IsPlay :type Boolean))
  (Variables|Default|Setisplay IsPlay)
  (return false))