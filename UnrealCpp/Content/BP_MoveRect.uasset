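; BP_MoveRect is an actor that moves its static mesh around a rectangular loop in the X-Z plane.
; While the flag set by DoPlay is true, Tick cycles MoveType through Right, Up, Left and Down.
; XPos and YPos act as time-driven step sizes added each frame, so the mesh speeds up on Right and Up, slows on Left and Down, and travels a frame-rate-dependent distance.
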(event EventTick
  (params (DeltaSeconds :type Float%20%28single-precision%29))
  (bind _staticmesh (Variables|Default|GetStaticMesh))
  (if (Variables|Default|Getplayg)
    (switch Utilities|FlowControl|Switch|SwitchonEN_MoveType (Variables|Default|GetMoveType)
      (:NewEnumerator0
        (bind _output_get (Variables|Default|SetX_pos (+ (Variables|Default|GetX_pos) DeltaSeconds)))
        (Transformation|AddRelativeLocation (Variables|Default|GetStaticMesh) (Math|Vector|MakeVector _output_get 0.0 0.0) false false)
        (if (>= (Variables|Default|GetX_pos) 2.0)
          (Variables|Default|SetMoveType "NewEnumerator1")))
      (:NewEnumerator1
        (bind _output_get_2 (Variables|Default|SetY_pos (+ (Variables|Default|GetY_pos) DeltaSeconds)))
        (Transformation|AddRelativeLocation (Variables|Default|GetStaticMesh) (Math|Vector|MakeVector 0.0 0.0 _output_get_2) false false)
        (if (>= (Variables|Default|GetY_pos) 2.0)
          (Variables|Default|SetMoveType "NewEnumerator2")))
      (:NewEnumerator2
        (bind _output_get_3 (Variables|Default|SetX_pos (- (Variables|Default|GetX_pos) DeltaSeconds)))
        (Transformation|AddRelativeLocation _staticmesh (Math|Vector|MakeVector (* _output_get_3 -1.0) 0.0 0.0) false false)
        (if (<= (Variables|Default|GetX_pos) 0.0)
          (Variables|Default|SetMoveType "NewEnumerator3")))
      (:NewEnumerator3
        (bind _output_get_4 (Variables|Default|SetY_pos (- (Variables|Default|GetY_pos) DeltaSeconds)))
        (Transformation|AddRelativeLocation _staticmesh (Math|Vector|MakeVector 0.0 0.0 (* _output_get_4 -1.0)) false false)
        (if (<= (Variables|Default|GetY_pos) 0.0)
          (Variables|Default|SetMoveType "NewEnumerator0"))))))

(fn ConstructionScript)

(fn DoPlay
  (params (IsPlay :type Boolean))
  (Variables|Default|Setplayg IsPlay)
  (return false))